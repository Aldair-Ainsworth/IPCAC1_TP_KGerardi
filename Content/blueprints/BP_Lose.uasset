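; BP_Lose is an actor that ends the game in a loss when any actor overlaps it.
; The overlap calls the Perder event, which prints a debug string and has MyHUD show the lose message.
; It then switches the first player controller to UI-only input, waits briefly and opens the MainMenu level.
; If the HUD cast fails, the sequence stops after the print.
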(event Custom|Perder
  (Development|PrintString "entro en perder")
  (bind _asmy_hud (Utilities|Casting|CastToMyHUD (HUD|GetHUD (Game|GetPlayerController 0))))
  (Default|MostrarMensajeLose _asmy_hud)
  (Input|SetInputModeUIOnly (Game|GetPlayerController 0) 0 "DoNotLock")
  (Utilities|FlowControl|Delay 2.0)
  (Game|OpenLevel(byName) "MainMenu"))

(event Collision|EventActorBeginOverlap
  (params (OtherActor :type Actor%20Object%20Reference))
  (CallFunction|Perder))

(fn ConstructionScript)