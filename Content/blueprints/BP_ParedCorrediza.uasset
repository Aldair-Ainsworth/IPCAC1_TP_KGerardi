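; BP_ParedCorrediza is a sliding wall that moves along the world Y axis once triggered.
; The Dezplazarse event sets the SeMueve flag, which is never cleared.
; While it is set, Tick moves the actor one unit per frame without sweep until its Y position reaches Distancia.
; Distancia acts as an absolute world coordinate rather than a travel offset, and the speed depends on frame rate.
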(event Custom|Dezplazarse
  (Variables|Default|SetSeMueve true))

(event EventTick
  (params (DeltaSeconds :type Float%20%28single-precision%29))
  (bind _returnvalue (Transformation|GetActorLocation))
  (bind (_x _y _z) (Math|Vector|BreakVector _returnvalue))
  (if (Variables|Default|GetSeMueve)
    (if (< _y (Math|Conversions|ToFloat(Integer) (Variables|Default|GetDistancia)))
      (Transformation|SetActorLocation (Math|Vector|MakeVector _x (+ _y 1.0) _z) false false))))

(fn ConstructionScript)