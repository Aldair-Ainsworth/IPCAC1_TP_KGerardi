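; BP_Aplastadora is a crusher hazard that oscillates vertically and ends the game on contact.
; Tick moves it one unit per frame without sweep, lowering it to Distancia and raising it via Restablecer to Distancia2, with CambiarDire toggling direction.
; A Trigger overlap checks only that MyPawn is valid, then calls Perder on MensajeLose, switches to UI-only input and opens MainMenu after a short delay.
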(event OnComponentBeginOverlap(Trigger)
  (params (OverlappedComponent :type Primitive%20Component%20Object%20Reference) (OtherActor :type Actor%20Object%20Reference) (OtherComp :type Primitive%20Component%20Object%20Reference) (OtherBodyIndex :type Integer) (bFromSweep :type Boolean) (SweepResult :type Hit%20Result%20Structure%20%28by%20ref%29))
  ;[1 1 1] Aplasto
  (Utilities|IsValid "/Game/blueprints/MyPawn.MyPawn"
    (:Is%20Valid
      (Default|Perder (Variables|Default|GetMensajeLose))
      (Input|SetInputModeUIOnly (Game|GetPlayerController 0) 0 "DoNotLock")
      (Utilities|FlowControl|Delay 2.0)
      (Game|OpenLevel(byName) "MainMenu"))))

(event Custom|Restablecer
  (bind _returnvalue (Transformation|GetActorLocation))
  (bind (_x _y _z) (Math|Vector|BreakVector _returnvalue))
  ;[1 1 1] Movimiento
  (if (< _z (Math|Conversions|ToFloat(Integer) (Variables|Default|GetDistancia2)))
    (Transformation|SetActorLocation (Math|Vector|MakeVector _x _y (+ _z 1.0)) false false)
    (else
      (Variables|Default|SetCambiarDire true))))

(event EventTick
  (params (DeltaSeconds :type Float%20%28single-precision%29))
  (bind _returnvalue (Transformation|GetActorLocation))
  (bind (_x _y _z) (Math|Vector|BreakVector _returnvalue))
  ;[1 1 1] Movimiento
  (if (Variables|Default|GetCambiarDire)
    (if (> _z (Math|Conversions|ToFloat(Integer) (Variables|Default|GetDistancia)))
      (Transformation|SetActorLocation (Math|Vector|MakeVector _x _y (- _z 1.0)) false false)
      (else
        (Variables|Default|SetCambiarDire false)))
    (else
      (CallFunction|Restablecer))))

(fn ConstructionScript)