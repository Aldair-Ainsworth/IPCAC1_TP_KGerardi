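; BP_BaladeCañon is a cannonball projectile that travels on its own and removes itself after a fixed lifetime.
; Each Tick adds a relative offset to its StaticMesh, mainly along X and derived from the world origin location, without sweep or delta-time scaling, so speed depends on frame rate.
; BeginPlay starts a delay that ends by destroying the actor.
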(event EventBeginPlay
  ;[1 1 1] Destruccion
  (Utilities|FlowControl|Delay 12.0)
  (Actor|DestroyActor))

(event EventTick
  (params (DeltaSeconds :type Float%20%28single-precision%29))
  (bind _returnvalue (Class|GameplayStatics|GetWorldOriginLocation))
  (bind _returnvalue_2 (Math|Conversions|ToVector(Float) _returnvalue))
  (bind (_x _y _z) (Math|Vector|BreakVector _returnvalue_2))
  ;[1 1 1] Movimiento
  (Transformation|AddRelativeLocation (Variables|Default|GetStaticMesh) (Math|Vector|MakeVector (* (+ _x 1.0) 3.0) _y _z) false false))

(fn ConstructionScript)