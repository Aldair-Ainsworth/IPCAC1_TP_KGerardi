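; MyHUD is a HUD Blueprint that shows the game's win and lose messages.
; On BeginPlay it creates MyWidget1 and MyWidget2, stores references to both and adds them to the viewport.
; MostrarMensajeWin calls MensajeWin on the first widget and MostrarMensajeLose calls MensajeLose on the second, each after a validity check.
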(event Custom|Mostrar%20Mensaje%20Lose
  (bind _refwidget2 (Variables|Default|GetRefWidget2))
  (Utilities|IsValid _refwidget2
    (:Is%20Valid
      (Default|MensajeLose _refwidget2))))

(event Custom|Mostrar%20Mensaje%20Win
  (bind _refwidget1 (Variables|Default|GetRefWidget1))
  (Utilities|IsValid _refwidget1
    (:Is%20Valid
      (Default|MensajeWin _refwidget1))))

(event EventBeginPlay
  (bind _returnvalue (UserInterface|CreateWidget "/Game/blueprints/MyWidget1.MyWidget1_C"))
  (bind _output_get (Variables|Default|SetRefWidget1 _returnvalue))
  (UserInterface|Viewport|AddtoViewport _output_get 0)
  (bind _returnvalue_2 (UserInterface|CreateWidget "/Game/blueprints/MyWidget2.MyWidget2_C"))
  (bind _output_get_2 (Variables|Default|SetRefWidget2 _returnvalue_2))
  (UserInterface|Viewport|AddtoViewport _output_get_2 0))

(fn ConstructionScript)